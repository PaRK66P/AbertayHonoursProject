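; Star collectible Blueprint that rewards the player with a star and points.
; It implements the CalculateCollectibles event, which increments the Stars count on ControllerReference and adds ScoreValue to its Score.
; BeginPlay is disabled and the construction script only calls its parent, so the file holds no other active logic.
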(event EventBeginPlay
  (|CallParentFunction) ; This node is disabled and will not be called.\nDrag off pins to build functionality.
)

(event EventCalculateCollectibles
  (bind _controllerreference (Variables|Default|GetControllerReference))
  (Variables|/Game/TemplateProject/_RainStoryGames/Blueprints/PC_Rainstory_Platformer.PC_Rainstory_Platformer_C|SetStars _controllerreference (+ (Variables|/Game/TemplateProject/_RainStoryGames/Blueprints/PC_Rainstory_Platformer.PC_Rainstory_Platformer_C|GetStars _controllerreference) 1))
  (Variables|/Game/TemplateProject/_RainStoryGames/Blueprints/PC_Rainstory_Platformer.PC_Rainstory_Platformer_C|SetScore _controllerreference (+ (Variables|/Game/TemplateProject/_RainStoryGames/Blueprints/PC_Rainstory_Platformer.PC_Rainstory_Platformer_C|GetScore _controllerreference) (Variables|Default|GetScoreValue))))

(fn ConstructionScript
  (|CallParentFunction))