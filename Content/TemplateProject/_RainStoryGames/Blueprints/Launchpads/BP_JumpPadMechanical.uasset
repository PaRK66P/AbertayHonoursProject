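; BP_JumpPadMechanical is a mechanical jump pad that launches characters who step onto it.
; Overlap with the pad mesh passes a DoOnce gate, plays a sound, then after a brief delay launches the BP_Character_Base with a velocity override and plays its jump montage.
; A timeline tilts the platform's scene component up, then reverses it and resets the gate on finish.
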(event OnComponentBeginOverlap(SM_Jumppad)
  (params (OverlappedComponent :type Primitive%20Component%20Object%20Reference) (OtherActor :type Actor%20Object%20Reference) (OtherComp :type Primitive%20Component%20Object%20Reference) (OtherBodyIndex :type Integer) (bFromSweep :type Boolean) (SweepResult :type Hit%20Result%20Structure%20%28by%20ref%29))
  (bind _asbp_character_base (Utilities|Casting|CastToBP_Character_Base OtherActor))
  (Utilities|FlowControl|DoOnce false
    (:Completed
      (Audio|PlaySound2D (Variables|Default|GetSound) 0.5 1.0 0.0 0 0)
      (Utilities|FlowControl|Delay 0.1)
      (Character|LaunchCharacter _asbp_character_base (Variables|Default|GetLaunch%20Velocity) true true)
      (CallFunction|RotatePad)
      (Default|PlayJumpMontage _asbp_character_base))))

(event Custom|RotatePad
  ;[1 1 1] Rotate the launch platform
  (bind _newtrack_0 (Timeline|Timeline Play)
    (:Update
      (Transformation|SetRelativeRotation (Variables|Default|GetScene) (Math|Rotator|Lerp(Rotator) "0.000000,0.000000,-5.000000" "0.000000,0.000000,45.000000" _newtrack_0) false false))
    (:Finished
      (CallFunction|ReturnPad)
      (Utilities|FlowControl|DoOnce false) ; enters at Reset
    )))

(event Custom|ReturnPad
  ;[1 1 1] Rotate the launch platform
  (bind _newtrack_0 (Timeline|Timeline Reverse)
    (:Update
      (Transformation|SetRelativeRotation (Variables|Default|GetScene) (Math|Rotator|Lerp(Rotator) "0.000000,0.000000,-5.000000" "0.000000,0.000000,45.000000" _newtrack_0) false false))
    (:Finished
      (CallFunction|ReturnPad)
      (Utilities|FlowControl|DoOnce false) ; enters at Reset
    )))

(fn ConstructionScript)