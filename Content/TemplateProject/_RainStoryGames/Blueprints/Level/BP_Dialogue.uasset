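; BP_Dialogue is a one-shot trigger that shows typewriter-style dialogue when an actor tagged Player first overlaps its Box.
; It plays a sound at its location, then creates a UI_Typewriter widget for the PC_Rainstory_Platformer controller with configurable text, color and typing speed.
; The widget's finished-writing callback waits for the RemoveAfter delay, then removes it from the screen.
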(event OnComponentBeginOverlap(Box)
  (params (OverlappedComponent :type Primitive%20Component%20Object%20Reference) (OtherActor :type Actor%20Object%20Reference) (OtherComp :type Primitive%20Component%20Object%20Reference) (OtherBodyIndex :type Integer) (bFromSweep :type Boolean) (SweepResult :type Hit%20Result%20Structure%20%28by%20ref%29))
  (if (Actor|ActorHasTag OtherActor "Player")
    (Utilities|FlowControl|DoOnce false
      (:Completed
        (CallFunction|CustomDialogue)))))

(event Custom|CustomEvent_3
  (Utilities|FlowControl|Delay (Variables|Default|GetRemoveAfter))
  (Widget|RemovefromParent (stale Custom|CustomDialogue _returnvalue)))

(event Custom|CustomDialogue
  (Audio|PlaySoundatLocation (Variables|Default|GetSound) (Transformation|GetWorldLocation (Variables|Default|GetDefaultSceneRoot)) "0, 0, 0" 1.0 1.0 0.0 0 0 0 0)
  (bind _aspc_rainstory_platformer (Utilities|Casting|CastToPC_Rainstory_Platformer (Game|GetPlayerController 0)))
  (bind _returnvalue (UserInterface|CreateWidget "/Game/TemplateProject/_RainStoryGames/Blueprints/UI/Typewriter/UI_Typewriter.UI_Typewriter_C" _aspc_rainstory_platformer (Variables|Default|GetCharacters%20Per%20Second) (Variables|Default|GetTextColor)))
  (UserInterface|Viewport|AddtoViewport _returnvalue 0)
  (Default|Write _returnvalue (Variables|Default|GetWriteText))
  (EventDispatchers|BindEventtoFinishedWriting _returnvalue (delegate Custom|CustomEvent_3)))

(fn ConstructionScript)