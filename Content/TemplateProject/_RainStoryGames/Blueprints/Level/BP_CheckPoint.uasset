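; Checkpoint actor for the platformer template that updates where the player spawns.
; On BeginPlay it caches the PC_Rainstory_Platformer player controller.
; The first capsule overlap by a Character tagged Player activates it once, turns its mesh translucent green and writes the SpawnPoint world transform to the controller's PlayerSpawnLocation.
; Activation also destroys the actor referenced as DestroyPreviousCheckpoint, if valid.
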(event OnComponentBeginOverlap(Capsule)
  (params (OverlappedComponent :type Primitive%20Component%20Object%20Reference) (OtherActor :type Actor%20Object%20Reference) (OtherComp :type Primitive%20Component%20Object%20Reference) (OtherBodyIndex :type Integer) (bFromSweep :type Boolean) (SweepResult :type Hit%20Result%20Structure%20%28by%20ref%29))
  (bind _destroypreviouscheckpoint (Variables|Default|GetDestroyPreviousCheckpoint))
  (if (not (Variables|Default|GetActivated))
    (bind _ascharacter (Utilities|Casting|CastToCharacter OtherActor))
    (if (Actor|ActorHasTag _ascharacter "Player")
      (Variables|Default|SetActivated true)
      (Rendering|Material|SetMaterial (Variables|Default|GetStaticMesh) 0 "/Game/TemplateProject/_RainStoryGames/Assets/Materials/MI_Translucent_Green.MI_Translucent_Green")
      (Variables|/Game/TemplateProject/_RainStoryGames/Blueprints/PC_Rainstory_Platformer.PC_Rainstory_Platformer_C|SetPlayerSpawnLocation (Variables|Default|GetControlerReference) (Transformation|GetWorldTransform (Variables|Default|GetSpawnPoint)))
      (Utilities|IsValid _destroypreviouscheckpoint
        (:Is%20Valid
          (Actor|DestroyActor _destroypreviouscheckpoint))))))

(event EventBeginPlay
  (bind _aspc_rainstory_platformer (Utilities|Casting|CastToPC_Rainstory_Platformer (Game|GetPlayerController 0)))
  (Variables|Default|SetControlerReference _aspc_rainstory_platformer))

(fn ConstructionScript)