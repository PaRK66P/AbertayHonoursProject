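; BP_DeathVolume is a kill volume that respawns a player character who touches it and costs them through a lives update.
; Overlapping its StaticMesh calls RespawnAtLocation (twice in succession) and UpdateLives on the BP_Character_Base, then runs FadeToBlack, which shows a UI_Fade widget for a second.
; A single DoOnce blocks repeat triggers until a character's end overlap resets it.
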(event OnComponentBeginOverlap(StaticMesh)
  (params (OverlappedComponent :type Primitive%20Component%20Object%20Reference) (OtherActor :type Actor%20Object%20Reference) (OtherComp :type Primitive%20Component%20Object%20Reference) (OtherBodyIndex :type Integer) (bFromSweep :type Boolean) (SweepResult :type Hit%20Result%20Structure%20%28by%20ref%29))
  (bind _asbp_character_base (Utilities|Casting|CastToBP_Character_Base OtherActor))
  (Utilities|FlowControl|DoOnce false
    (:Completed
      (Default|RespawnatLocation _asbp_character_base)
      (Default|RespawnatLocation _asbp_character_base)
      (Default|UpdateLives _asbp_character_base)
      (CallFunction|FadetoBlack))))

(event OnComponentEndOverlap(StaticMesh)
  (params (OverlappedComponent :type Primitive%20Component%20Object%20Reference) (OtherActor :type Actor%20Object%20Reference) (OtherComp :type Primitive%20Component%20Object%20Reference) (OtherBodyIndex :type Integer))
  (Utilities|Casting|CastToBP_Character_Base OtherActor)
  (Utilities|FlowControl|DoOnce false) ; enters at Reset
)

(event Custom|FadeToBlack
  (bind _returnvalue (UserInterface|CreateWidget "/Game/TemplateProject/_RainStoryGames/Blueprints/UI/UI_Fade.UI_Fade_C"))
  (UserInterface|Viewport|AddtoViewport _returnvalue 0)
  (Utilities|FlowControl|Delay 1.0)
  (Widget|RemovefromParent _returnvalue))

(fn ConstructionScript)