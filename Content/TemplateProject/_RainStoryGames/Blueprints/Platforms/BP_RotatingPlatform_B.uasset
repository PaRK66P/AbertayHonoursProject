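; Rotating platform actor that flips back and forth between 0 and 180 degrees in a continuous loop.
; On BeginPlay, if AutoStart is set, it waits DelayStart, then RotateA and RotateB alternate endlessly, pausing Interval between each turn.
; Each half uses its own Timeline MoveTrack to lerp the root component's relative rotation on one axis.
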(event Custom|RotateB
  (bind _movetrack (Timeline|Timeline_0 PlayFromStart)
    (:Update
      (Transformation|SetRelativeRotation (Variables|Default|GetDefaultSceneRoot) (Math|Rotator|Lerp(Rotator) "180.000000,0.000000,0.000000" "0, 0, 0" _movetrack) false false))
    (:Finished
      (Utilities|FlowControl|Delay (Variables|Default|GetInterval))
      (CallFunction|RotateA))))

(event Custom|RotateA
  (bind _movetrack (Timeline|Timeline PlayFromStart)
    (:Update
      (Transformation|SetRelativeRotation (Variables|Default|GetDefaultSceneRoot) (Math|Rotator|Lerp(Rotator) "0, 0, 0" "180.000000,0.000000,0.000000" _movetrack) false false))
    (:Finished
      (Utilities|FlowControl|Delay (Variables|Default|GetInterval))
      (CallFunction|RotateB))))

(event EventBeginPlay
  (if (Variables|Default|GetAutoStart)
    (Utilities|FlowControl|Delay (Variables|Default|GetDelayStart))
    (CallFunction|RotateA)))

(fn ConstructionScript)