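; Platform actor that moves toward an end position when a Player-tagged Character overlaps it and returns when that character steps off.
; A timeline, with play rate scaled by DurationInSeconds, lerps MainPlatform's relative location from its start to EndPlatformReference's location, reversing on end overlap.
; The construction script applies one configurable mesh to the platform, collision trigger and end marker, giving the latter two translucent materials.
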(event OnComponentBeginOverlap(MeshCollision)
  (params (OverlappedComponent :type Primitive%20Component%20Object%20Reference) (OtherActor :type Actor%20Object%20Reference) (OtherComp :type Primitive%20Component%20Object%20Reference) (OtherBodyIndex :type Integer) (bFromSweep :type Boolean) (SweepResult :type Hit%20Result%20Structure%20%28by%20ref%29))
  (bind _ascharacter (Utilities|Casting|CastToCharacter OtherActor))
  (if (Actor|ActorHasTag _ascharacter "Player")
    (Components|Timeline|SetPlayRate (Variables|Default|GetMovePlatform) (/ 1.0 (Variables|Default|GetDurationInSeconds)))
    (bind _movetrack (Timeline|MovePlatform Play)
      (:Update
        (Transformation|SetRelativeLocation (Variables|Default|GetMainPlatform) (Math|Vector|Lerp(Vector) (Variables|Default|GetStartLocation) (Variables|Default|GetEndLocation) _movetrack) false false)))))

(event OnComponentEndOverlap(MeshCollision)
  (params (OverlappedComponent :type Primitive%20Component%20Object%20Reference) (OtherActor :type Actor%20Object%20Reference) (OtherComp :type Primitive%20Component%20Object%20Reference) (OtherBodyIndex :type Integer))
  (bind _ascharacter (Utilities|Casting|CastToCharacter OtherActor))
  (if (Actor|ActorHasTag _ascharacter "Player")
    (Components|Timeline|SetPlayRate (Variables|Default|GetMovePlatform) (/ 1.0 (Variables|Default|GetDurationInSeconds)))
    (bind _movetrack (Timeline|MovePlatform Reverse)
      (:Update
        (Transformation|SetRelativeLocation (Variables|Default|GetMainPlatform) (Math|Vector|Lerp(Vector) (Variables|Default|GetStartLocation) (Variables|Default|GetEndLocation) _movetrack) false false)))))

(event Custom|ReturnToStart
  (Components|Timeline|SetPlayRate (Variables|Default|GetMovePlatform) (/ 1.0 (Variables|Default|GetDurationInSeconds)))
  (bind _movetrack (Timeline|MovePlatform Reverse)
    (:Update
      (Transformation|SetRelativeLocation (Variables|Default|GetMainPlatform) (Math|Vector|Lerp(Vector) (Variables|Default|GetStartLocation) (Variables|Default|GetEndLocation) _movetrack) false false))))

(event Custom|MoveToLocation
  (Components|Timeline|SetPlayRate (Variables|Default|GetMovePlatform) (/ 1.0 (Variables|Default|GetDurationInSeconds)))
  (bind _movetrack (Timeline|MovePlatform Play)
    (:Update
      (Transformation|SetRelativeLocation (Variables|Default|GetMainPlatform) (Math|Vector|Lerp(Vector) (Variables|Default|GetStartLocation) (Variables|Default|GetEndLocation) _movetrack) false false))))

(event EventBeginPlay
  (Variables|Default|SetStartLocation (Variables|/Script/Engine.SceneComponent|GetRelativeLocation (Variables|Default|GetMainPlatform)))
  (Variables|Default|SetEndLocation (Variables|/Script/Engine.SceneComponent|GetRelativeLocation (Variables|Default|GetEndPlatformReference))))

(fn ConstructionScript
  (bind _meshcollision (Variables|Default|GetMeshCollision))
  (bind _endplatformreference (Variables|Default|GetEndPlatformReference))
  (bind _platformmesh (Variables|Default|GetPlatformMesh))
  (Components|StaticMesh|SetStaticMesh (Variables|Default|GetMainPlatform) _platformmesh)
  (Components|StaticMesh|SetStaticMesh _meshcollision _platformmesh)
  (Rendering|Material|SetMaterial _meshcollision 0 "/Game/TemplateProject/_RainStoryGames/Assets/Materials/MI_Translucent_Mesh.MI_Translucent_Mesh")
  (Components|StaticMesh|SetStaticMesh _endplatformreference _platformmesh)
  (Rendering|Material|SetMaterial _endplatformreference 0 "/Game/TemplateProject/_RainStoryGames/Assets/Materials/MI_Translucent_Yellow.MI_Translucent_Yellow"))