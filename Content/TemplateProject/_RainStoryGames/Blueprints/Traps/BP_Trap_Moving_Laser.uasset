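; Laser trap Blueprint that moves along a set path and damages characters that touch it.
; The construction script copies the control points and duration into an InterpToMovement component and applies the configurable laser mesh, so each instance can define its own path, timing and look.
; When the mesh begins overlapping a BP_Character_Base, the trap applies a small fixed damage to it with itself as the damage causer.
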(event OnComponentBeginOverlap(StaticMesh)
  (params (OverlappedComponent :type Primitive%20Component%20Object%20Reference) (OtherActor :type Actor%20Object%20Reference) (OtherComp :type Primitive%20Component%20Object%20Reference) (OtherBodyIndex :type Integer) (bFromSweep :type Boolean) (SweepResult :type Hit%20Result%20Structure%20%28by%20ref%29))
  (bind _asbp_character_base (Utilities|Casting|CastToBP_Character_Base OtherActor))
  (Game|Damage|ApplyDamage _asbp_character_base 1.0 0 self))

(fn ConstructionScript
  (bind _interptomovement (Variables|Default|GetInterpToMovement))
  (Variables|/Script/Engine.InterpToMovementComponent|SetControlPoints _interptomovement (Variables|Default|GetControl%20Points))
  (Variables|/Script/Engine.InterpToMovementComponent|SetDuration _interptomovement (Variables|Default|GetDuration))
  (Components|StaticMesh|SetStaticMesh (Variables|Default|GetStaticMesh) (Variables|Default|GetLaserMesh)))