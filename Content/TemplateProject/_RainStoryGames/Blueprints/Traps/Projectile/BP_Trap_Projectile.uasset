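; Trap projectile actor that damages actors tagged Player when it hits them.
; A sound plays at its Sphere component on BeginPlay.
; On a player hit it applies damage, spawns an emitter and plays an attenuated sound at the impact point, then destroys itself.
; Any other hit only spawns an impact emitter before destroying it.
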(event EventBeginPlay
  (Audio|PlaySoundatLocation 0 (Transformation|GetWorldLocation (Variables|Default|GetSphere)) "0, 0, 0" 1.0 1.0 0.0 0 0 0 0))

(event Collision|EventHit
  (params (MyComp :type Primitive%20Component%20Object%20Reference) (Other :type Actor%20Object%20Reference) (OtherComp :type Primitive%20Component%20Object%20Reference) (bSelfMoved :type Boolean) (HitLocation :type Vector :default "0, 0, 0") (HitNormal :type Vector :default "0, 0, 0") (NormalImpulse :type Vector :default "0, 0, 0") (Hit :type Hit%20Result%20Structure%20%28by%20ref%29))
  (bind (_bblockinghit _binitialoverlap _time _distance _location _impactpoint _normal _impactnormal _physmat _hitactor) (Collision|BreakHitResult Hit))
  (if (Actor|ActorHasTag Other "Player")
    (Game|Damage|ApplyDamage Other (Variables|Default|GetBase%20Damage) 0 0 "/Script/Engine.DamageType")
    (Effects|SpawnEmitteratLocation 0 _impactpoint (.rotation (Transformation|GetActorTransform _hitactor)))
    (Audio|PlaySoundatLocation 0 _impactpoint "0, 0, 0" 0.5 1.0 0.0 "/Game/TemplateProject/_RainStoryGames/Blueprints/Traps/Projectile/ProjectileSoundAttenuation.ProjectileSoundAttenuation" 0 0 0)
    (Utilities|IsValid self
      (:Is%20Valid
        (Actor|DestroyActor)))
    (else
      (Effects|SpawnEmitteratLocation 0 (.ImpactPoint (Collision|BreakHitResult Hit)))
      (Actor|DestroyActor))))

(fn ConstructionScript)