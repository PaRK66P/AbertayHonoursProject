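; Projectile trap that fires when a player-tagged actor enters its trigger box.
; A DoOnce gate allows one shot per entry and resets when the player leaves the box.
; Each shot turns an emissive material red, waits briefly, then spawns a BP_Trap_Projectile along the Arrow's forward vector with particle and sound effects, and restores the blue material.
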(event OnComponentBeginOverlap(Box)
  (params (OverlappedComponent :type Primitive%20Component%20Object%20Reference) (OtherActor :type Actor%20Object%20Reference) (OtherComp :type Primitive%20Component%20Object%20Reference) (OtherBodyIndex :type Integer) (bFromSweep :type Boolean) (SweepResult :type Hit%20Result%20Structure%20%28by%20ref%29))
  (if (Actor|ActorHasTag OtherActor "Player")
    (Utilities|FlowControl|DoOnce false
      (:Completed
        (CallFunction|ShootProjectile)))))

(event OnComponentEndOverlap(Box)
  (params (OverlappedComponent :type Primitive%20Component%20Object%20Reference) (OtherActor :type Actor%20Object%20Reference) (OtherComp :type Primitive%20Component%20Object%20Reference) (OtherBodyIndex :type Integer))
  (if (Actor|ActorHasTag OtherActor "Player")
    (Utilities|FlowControl|DoOnce false) ; enters at Reset
  ))

(event Custom|ShootProjectile
  (bind _arrow (Variables|Default|GetArrow))
  (bind _returnvalue (Transformation|GetWorldLocation _arrow))
  (Rendering|Material|SetMaterial (Variables|Default|GetStaticMesh) 1 "/Game/TemplateProject/_RainStoryGames/Assets/Materials/MI_Emissive_Red.MI_Emissive_Red")
  (Utilities|FlowControl|Delay 0.5)
  (Effects|SpawnEmitteratLocation 0 (Transformation|GetWorldLocation (Variables|Default|GetArrow)))
  (Game|SpawnActorfromClass "/Game/TemplateProject/_RainStoryGames/Blueprints/Traps/Projectile/BP_Trap_Projectile.BP_Trap_Projectile_C" (Math|Transform|MakeTransform _returnvalue (Math|Conversions|RotationFromXVector (Math|Vector|GetForwardVector _arrow)) (Variables|Default|GetScale)) "Undefined" "OverrideRootScale" self 0)
  (Audio|SpawnSoundatLocation 0 _returnvalue "0, 0, 0" 1.0 1.0 0.0 "/Game/TemplateProject/_RainStoryGames/Blueprints/Traps/Projectile/ProjectileSoundAttenuation.ProjectileSoundAttenuation" 0)
  (Rendering|Material|SetMaterial (Variables|Default|GetStaticMesh) 1 "/Game/TemplateProject/_RainStoryGames/Assets/Materials/MI_Emissive_Blue.MI_Emissive_Blue"))

(fn ConstructionScript)