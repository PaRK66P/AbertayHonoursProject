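; BP_RotatingLaser is a trap that spins a laser and damages characters that touch it.
; At BeginPlay, the Oposite flag selects one of two rotation rates for its RotatingMovement component.
; The construction script applies LaserMesh to CollisionMesh, whose begin-overlap event applies fixed damage to any BP_Character_Base.
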(event OnComponentBeginOverlap(CollisionMesh)
  (params (OverlappedComponent :type Primitive%20Component%20Object%20Reference) (OtherActor :type Actor%20Object%20Reference) (OtherComp :type Primitive%20Component%20Object%20Reference) (OtherBodyIndex :type Integer) (bFromSweep :type Boolean) (SweepResult :type Hit%20Result%20Structure%20%28by%20ref%29))
  (bind _asbp_character_base (Utilities|Casting|CastToBP_Character_Base OtherActor))
  (Game|Damage|ApplyDamage _asbp_character_base 1.0 0 self))

(event EventBeginPlay
  (bind _rotatingmovement (Variables|Default|GetRotatingMovement))
  (if (Variables|Default|GetOposite)
    (Variables|/Script/Engine.RotatingMovementComponent|SetRotationRate _rotatingmovement (Variables|Default|GetRotateA))
    (else
      (Variables|/Script/Engine.RotatingMovementComponent|SetRotationRate _rotatingmovement (Variables|Default|GetRotateB)))))

(fn ConstructionScript
  (Components|StaticMesh|SetStaticMesh (Variables|Default|GetCollisionMesh) (Variables|Default|GetLaserMesh)))