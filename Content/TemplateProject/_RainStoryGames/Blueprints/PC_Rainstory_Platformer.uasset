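; Player controller for a platformer template that handles level setup, collectible totals, level timing and failure.
; BeginPlay applies performance settings, counts placed coins and stars for the UI and sets game-only input; HUD creation is left disconnected.
; Two Timelines drive a timer and a reverse-played countdown, both updating the time text.
; When the countdown finishes, LevelFail pauses the game and shows the failure widget, while Escape opens the main menu.
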(event Custom|EndTimer
  ;[1 1 1] Timer
  (bind _leveltimer (Timeline|Timeline Stop)
    (:Update
      (bind _output_get (Variables|Default|SetLevel%20Time%20Countdown _leveltimer))
      (Variables|Default|SetLevelCountdownText (Utilities|TimetoText _output_get)))))

(event Custom|StartTimer
  ;[1 1 1] Timer
  (bind _leveltimer (Timeline|Timeline PlayFromStart)
    (:Update
      (bind _output_get (Variables|Default|SetLevel%20Time%20Countdown _leveltimer))
      (Variables|Default|SetLevelCountdownText (Utilities|TimetoText _output_get)))))

(event Custom|CheckCoinsCount
  ;[1 1 1] Check for all the collectibles in the level and prepare it for the UI Widget
  (bind _outactors (Actor|GetAllActorsOfClass "/Game/TemplateProject/_RainStoryGames/Blueprints/Collectibles/BP_Collectible_Coins.BP_Collectible_Coins_C"))
  (Variables|Default|SetCoins_Count (Utilities|Array|Length _outactors)))

(event Custom|CheckStarsCount
  ;[1 1 1] Check for all the collectibles in the level and prepare it for the UI Widget
  (bind _outactors (Actor|GetAllActorsOfClass "/Game/TemplateProject/_RainStoryGames/Blueprints/Collectibles/BP_Collectible_Stars.BP_Collectible_Stars_C"))
  (Variables|Default|SetStars_Count (Utilities|Array|Length _outactors)))

(event Custom|LevelFail
  (bind _returnvalue (Game|GetPlayerController 0))
  (Variables|Default|SetLevelFailed true)
  (Utilities|FlowControl|Delay 0.2)
  (Game|SetGamePaused true)
  (Variables|/Script/Engine.PlayerController|SetbShowMouseCursor _returnvalue true)
  (bind _returnvalue_2 (UserInterface|CreateWidget "/Game/TemplateProject/_RainStoryGames/Blueprints/UI/UI_LevelFailed.UI_LevelFailed_C"))
  (UserInterface|Viewport|AddtoViewport _returnvalue_2 0)
  (Input|SetInputModeUIOnly _returnvalue _returnvalue_2 "DoNotLock" false))

(event Custom|StartCountdown
  ;[1 1 1] Countdown and end game if the timer reaches 0
  (bind _leveltimer (Timeline|CountedownTimeline ReverseFromEnd)
    (:Update
      (bind _output_get (Variables|Default|SetLevel%20Time%20Countdown _leveltimer))
      (Variables|Default|SetLevelCountdownText (Utilities|TimetoText _output_get)))
    (:Finished
      (CallFunction|EndGameonCountdown))))

(event Custom|EndCountdown
  ;[1 1 1] Countdown and end game if the timer reaches 0
  (bind _leveltimer (Timeline|CountedownTimeline Stop)
    (:Update
      (bind _output_get (Variables|Default|SetLevel%20Time%20Countdown _leveltimer))
      (Variables|Default|SetLevelCountdownText (Utilities|TimetoText _output_get)))
    (:Finished
      (CallFunction|EndGameonCountdown))))

(event Custom|EndGameOnCountdown
  ;[1 1 1] Countdown and end game if the timer reaches 0
  (CallFunction|EndCountdown)
  (CallFunction|LevelFail))

(event EventBeginPlay
  (bind _returnvalue (Game|GetPlayerController 0))
  (Utilities|FlowControl|Sequence
    (:then_0
      (Development|ExecuteConsoleCommand "t.maxfps 60" 0)
      (Development|ExecuteConsoleCommand "r.ScreenPercentage 70" 0)
      (bind _returnvalue_2 (Settings|GetGameUserSettings))
      (Class|GameUserSettings|SetGlobalIlluminationQuality _returnvalue_2))
    (:then_1
      (CallFunction|CheckCoinsCount)
      (CallFunction|CheckStarsCount))
    (:then_2
      (Variables|/Script/Engine.PlayerController|SetbShowMouseCursor _returnvalue false)
      (Input|SetInputModeGameOnly _returnvalue false))))

(event Input|KeyboardEvents|Escape
  (params (Key :type Key%20Structure :default "None"))
  (:Pressed
    (Game|OpenLevel(byName) "L_MainMenu")))

(fn ConstructionScript)